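; MP5 weapon for the BP_FPS player, with its stats set in the construction script and its state saved to the SecondaryWeapon slot on unequip.
; Fire spends ammo, applies damage via a camera-centre hitscan, then spawns a decal, occasional tracer and muzzle flash; empty fire plays a dry-fire sound.
; Reload plays arm and gun animations, refilling after a delay behind a DoOnce.
; The gun's fire animation is an AK asset, Arms_AK_Fire_anim.
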(event `self.Unequip`
  (set `/Game/Blueprints/Characters/Player/BP_FPS.SecondaryWeapon` (make `/Game/Blueprints/Weapons/GunData` "NewEnumerator3" "BP_Weapon_MP5_C" (`self.AmmoCount`) (`self.MaxAmmo`) (`self.ReloadTime`) (`self.BulletSpread`)) (cast `/Game/Blueprints/Characters/Player/BP_FPS` (`GameplayStatics.GetPlayerCharacter` 0) :!pure true)))

(event `self.Fire`
  ;[1 1 1] Shoot AK47
  (if (> (`self.AmmoCount`) 0)
    (`self.AmmoCheck`)
    (bind (_muzzleloc _impactpoint) (`self.LineTrace`))
    (`self.SpawnDecalTracer` _muzzleloc _impactpoint _impactpoint)
    (`|PlayMontage` (`/Game/Blueprints/Characters/Player/BP_FPS.Mesh2P` (cast `/Game/Blueprints/Characters/Player/BP_FPS` (`GameplayStatics.GetPlayerCharacter` 0) :!pure true)) "/Game/Animations/MP5/Arms_MP5_Fire_anim_Montage.Arms_MP5_Fire_anim_Montage"
      (:`then`
        (`self.MuzzleFlash`)))
    (else
      (`GameplayStatics.PlaySoundAtLocation` "/Game/Audio/weapons/DryFire.DryFire" (`self.K2_GetActorLocation`) (struct) 1.0 1.0 0.0 null null null))))

(event `self.Reload`
  (bind _asbp_fps (cast `/Game/Blueprints/Characters/Player/BP_FPS` (`GameplayStatics.GetPlayerCharacter` 0) :!pure true))
  ;[1 1 1] Reload AK47
  (if (< (`self.AmmoCount`) (`self.MaxAmmo`))
    (`/Engine/EditorBlueprintResources/StandardMacros.DoOnce` false :!label _label
      (:`Completed`
        (set `/Game/Blueprints/Characters/Player/BP_FPS.IsReloading?` true _asbp_fps)
        (`AnimInstance.Montage_Play` (`SkeletalMeshComponent.GetAnimInstance` (`/Game/Blueprints/Characters/Player/BP_FPS.Mesh2P` _asbp_fps)) "/Game/Animations/MP5/Arms_MP5_Reload_anim_Montage.Arms_MP5_Reload_anim_Montage" 1.0 "MontageLength" 0.0 true)
        (`SkeletalMeshComponent.PlayAnimation` (`self.PrimaryWeapon`) "/Game/Animations/MP5/MP5_Reload_anim.MP5_Reload_anim" false)
        (`KismetSystemLibrary.Delay` (`self.ReloadTime`))
        (set `self.AmmoCount` (`self.MaxAmmo`))
        (set `/Game/Blueprints/Characters/Player/BP_FPS.IsReloading?` false _asbp_fps)
        (goto _label :!via `Reset`)))))

(fn `AmmoCheck`
  (bind _returnvalue (`KismetMathLibrary.RandomFloatInRange` 0.6 0.9))
  (`/Engine/EditorBlueprintResources/StandardMacros.DecrementInt` (`self.AmmoCount`)
    (:`  `
      (`GameplayStatics.PlaySoundAtLocation` "/Game/Audio/weapons/Gunshot.Gunshot" (`self.K2_GetActorLocation`) (struct) (+ _returnvalue 2.8) _returnvalue 0.0 null null null)
      (`SkeletalMeshComponent.PlayAnimation` (`self.PrimaryWeapon`) "/Game/Animations/AK47/Arms_AK_Fire_anim.Arms_AK_Fire_anim" false))))

(fn `LineTrace`
  (returns (MuzzleLoc :type "Vector Structure") (ImpactPoint :type "Vector Structure"))
  (bind _returnvalue (`SceneComponent.K2_GetComponentLocation` (`self.Muzzle`)))
  (bind _firstpersoncamera (`/Game/Blueprints/Characters/Player/BP_FPS.FirstPersonCamera` (cast `/Game/Blueprints/Characters/Player/BP_FPS` (`GameplayStatics.GetPlayerCharacter` 0) :!pure true)))
  (bind _returnvalue_2 (`SceneComponent.K2_GetComponentLocation` _firstpersoncamera))
  (bind _outhit (`KismetSystemLibrary.LineTraceSingle` _returnvalue_2 (+ _returnvalue_2 (* (`SceneComponent.GetForwardVector` _firstpersoncamera) 20000.0)) "TraceTypeQuery1")) ; Camera Shot
  (bind (_bblockinghit _binitialoverlap _time _distance _location _impactpoint _normal _impactnormal _physmat _hitactor) (`GameplayStatics.BreakHitResult` _outhit))
  (`GameplayStatics.ApplyDamage` _hitactor (`self.BaseDamage`))
  (`KismetSystemLibrary.LineTraceSingle` :`Start` _returnvalue :`End` _impactpoint :`TraceChannel` "TraceTypeQuery1" :`TraceColor` (struct :`R` 0.008226 :`G` 1.0 :`B` 0.107856 :`A` 1.0)) ; Camera Shot
  (return _returnvalue _impactpoint))

(fn `SpawnDecalTracer`
  (params (Location :type "Vector Structure") (SpawnTransformLoc :type "Vector Structure") (ImpactPoint :type "Vector Structure"))
  (`|SpawnActorFromClass` "/Game/Blueprints/Weapons/BP_BulletDecal.BP_BulletDecal_C" (`KismetMathLibrary.MakeTransform` SpawnTransformLoc (`KismetMathLibrary.Conv_VectorToRotator` ImpactPoint) (0.025 0.025 0.025)) "Undefined" "OverrideRootScale" null null)
  (if (>= (`KismetMathLibrary.RandomIntegerInRange` 1 10) 7)
    (`|SpawnActorFromClass` "/Game/Blueprints/Weapons/BP_TracerRounds.BP_TracerRounds_C" (`KismetMathLibrary.MakeTransform` Location (`SceneComponent.K2_GetComponentRotation` (`/Game/Blueprints/Characters/Player/BP_FPS.FirstPersonCamera` (cast `/Game/Blueprints/Characters/Player/BP_FPS` (`GameplayStatics.GetPlayerCharacter` 0) :!pure true))) (0.3 0.3 0.3)) "Undefined" "OverrideRootScale" null null))
  (return))

(fn `UserConstructionScript`
  (`parent.UserConstructionScript`)
  (set `self.MaxAmmo` 18)
  (set `self.AmmoCount` 18)
  (set `self.ReloadTime` 1.8)
  (set `self.BulletSpread` 0.0)
  (set `self.Name` "NewEnumerator3")
  (set `self.BaseDamage` 25.0))