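; BP_PickUp_MP51 is an inventory pickup Blueprint, apparently for an MP5, that launches itself when it spawns.
; On BeginPlay it casts the player character to BP_FPS and applies that character's DropImpulse to its Capsule as a velocity change, so mass is ignored.
; The construction script only calls the parent; overlap, tick and the parent BeginPlay call are disabled, and no pickup logic is defined in these graphs.
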(event `self.ReceiveBeginPlay`
  (bind _asbp_fps (cast `/Game/Blueprints/Characters/Player/BP_FPS` (`GameplayStatics.GetPlayerCharacter` 0)))
  (`PrimitiveComponent.AddImpulse` (`self.Capsule`) (`/Game/Blueprints/Characters/Player/BP_FPS.DropImpulse` _asbp_fps) "None" true))

(fn `UserConstructionScript`
  (`parent.UserConstructionScript`))