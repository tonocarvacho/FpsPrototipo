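; NPC actor that shows dialogue line by line from the Dialogue data table when interacted with.
; BeginPlay caches the rows matching its NPCID, and each Interact advances the line counter and creates or updates the UI_Dialog widget.
; DialogueGetLine matches conversation and line IDs, closing the widget and resetting the counter unless exactly one line is found.
; Ending overlap also closes and resets an open dialogue.
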(event `self.ReceiveBeginPlay`
  (bind _outrownames (`DataTableFunctionLibrary.GetDataTableRowNames` "/Game/Blueprints/HUD/Dialogue/Dialogue.Dialogue"))
  (for _array_element _outrownames
    (bind _returnvalue (`|GetDataTableRow` "/Game/Blueprints/HUD/Dialogue/Dialogue.Dialogue" _array_element)
      (:`then`
        (if (== (`.NPC_ID_2_EFAC1DDC4801DBC5CECB319CAEA02DE5` (break `/Game/Blueprints/HUD/Dialogue/S_DialogueData` _returnvalue)) (`self.NPC_ID`))
          (`KismetArrayLibrary.Array_Add` (`self.MyDialogue`) _array_element))))))

(event `/Game/Blueprints/HUD/Dialogue/BP_DialogInterface.Interact`
  (`/Engine/EditorBlueprintResources/StandardMacros.IncrementInt` (`self.LineCurrent`)
    (:`  `
      (`self.DialogueCreate`))))

(event `self.ReceiveActorEndOverlap`
  (params (OtherActor :type "Actor Object Reference"))
  (`/Engine/EditorBlueprintResources/StandardMacros.IsValid` (`self.UIDialogRef`)
    (:`Is Valid`
      (`Widget.RemoveFromParent` (`self.UIDialogRef`))
      (set `self.UIDialogRef` null)
      (set `self.LineCurrent` 0))))

(fn `DialogueCreate`
  (bind _uidialogref (`self.UIDialogRef`))
  (`/Engine/EditorBlueprintResources/StandardMacros.IsValid` (`self.UIDialogRef`)
    (:`Is Valid`
      (bind _returnedline (`self.DialogueGetLine`))
      (`/Engine/EditorBlueprintResources/StandardMacros.IsValid` _uidialogref
        (:`Is Valid`
          (set `/Game/Blueprints/HUD/Dialogue/UI_Dialog.DialogueText` _returnedline _uidialogref))))
    (:`Is Not Valid`
      (bind _returnvalue (`|CreateWidget` "/Game/Blueprints/HUD/Dialogue/UI_Dialog.UI_Dialog_C" (`GameplayStatics.GetPlayerController` 0)))
      (bind _output_get (set `self.UIDialogRef` _returnvalue))
      (`UserWidget.AddToViewport` _output_get 0)
      (bind _returnedline_2 (`self.DialogueGetLine`))
      (set `/Game/Blueprints/HUD/Dialogue/UI_Dialog.DialogueText` _returnedline_2 (`self.UIDialogRef`)))))

(fn `DialogueGetLine`
  (returns (ReturnedLine :type Text))
  (locals (LineReturned :type "Array of Text"))
  (for _array_element (`self.MyDialogue`)
    (bind _returnvalue (`|GetDataTableRow` "/Game/Blueprints/HUD/Dialogue/Dialogue.Dialogue" _array_element)
      (:`then`
        (bind (_npc_id _conversation_id _line_id _dialogue) (break `/Game/Blueprints/HUD/Dialogue/S_DialogueData` _returnvalue))
        (if (and (== _conversation_id (`self.Conversation_ID`)) (== _line_id (`self.LineCurrent`)))
          (`KismetArrayLibrary.Array_Add` (`local.LineReturned`) _dialogue)))))
  (if (== (`KismetArrayLibrary.Array_Length` (`local.LineReturned`)) 1)
    (return (`|GetArrayItem` (`local.LineReturned`)))
    (else
      (`Widget.RemoveFromParent` (`self.UIDialogRef`))
      (set `/Game/Blueprints/HUD/Dialogue/UI_Dialog.DialogueText` "" (`self.UIDialogRef`))
      (set `self.UIDialogRef` null)
      (set `self.LineCurrent` 0))))

(fn `UserConstructionScript`)