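; BP_Enemy_Alien is an alien enemy that faces pawns it sees, fires cooldown-gated projectiles and repeatedly damages the player while overlapping.
; BeginPlay selects roam or chase from AIstate, but both events are empty, with their AIMoveTo logic left disconnected.
; Player death disables pawn sensing and re-runs that state switch.
; When its health runs out, the alien destroys itself and makes all BP_PointLight lights visible.
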(event `self.ReceiveBeginPlay`
  (bind _asbp_fps (cast `/Game/Blueprints/Characters/Player/BP_FPS` (`GameplayStatics.GetPlayerCharacter` 0)))
  (add `/Game/Blueprints/Characters/Player/BP_FPS.PlayerDied` _asbp_fps (delegate `ResetAi`))
  (switch `/Game/Blueprints/Characters/NPCs/E_AIState` (`self.AIstate`) :!label _label
    (:`NewEnumerator0`
      (`self.MoveToRandomLocation`))
    (:`NewEnumerator1`
      (`self.MoveToRandomLocation`))
    (:`NewEnumerator2`
      (`self.ChasePlayer`))))

(event `ResetAi`
  (`PawnSensingComponent.SetSensingUpdatesEnabled` (`self.PawnSensing`) false)
  (goto _label))

(event `self.ReceiveAnyDamage`
  (params (Damage :type "Float (single-precision)") (DamageType :type "DamageType Object Reference") (InstigatedBy :type "Controller Object Reference") (DamageCauser :type "Actor Object Reference"))
  ;[1 1 1] dano
  (if (> (`self.CurrentHealth`) 0.0)
    (bind _output_get (set `self.CurrentHealth` (- (`self.CurrentHealth`) Damage)))
    (if (<= _output_get 0.0)
      (`self.K2_DestroyActor`)
      (bind _outactors (`GameplayStatics.GetAllActorsOfClass` "/Game/Blueprints/Objects/BP_PointLight.BP_PointLight_C"))
      (for _array_element _outactors
        (`SceneComponent.SetVisibility` (`/Game/Blueprints/Objects/BP_PointLight.PointLight` _array_element) true false)))))

(event `ChasePlayer`)

(event `MoveToRandomLocation`)

(event `self.ReceiveActorBeginOverlap`
  (params (OtherActor :type "Actor Object Reference"))
  (bind _returnvalue (`GameplayStatics.GetPlayerCharacter` 0))
  (if (`self.IsOverlappingActor` _returnvalue) :!label _label_2
    (`GameplayStatics.ApplyDamage` (cast `/Game/Blueprints/Characters/Player/BP_FPS` _returnvalue :!pure true) (`self.AppliedDamage`))
    (`KismetSystemLibrary.Delay` 0.5)
    (goto _label_2)))

(event `self.PawnSensing.OnSeePawn`
  (params (Pawn :type "Pawn Object Reference"))
  (bind _ascharacter (cast `Character` Pawn))
  (`|ExecutionSequence`
    (:`then_0`
      (`self.K2_SetActorRotation` (`KismetMathLibrary.FindLookAtRotation` (`self.K2_GetActorLocation`) (`self.K2_GetActorLocation` _ascharacter))))
    (:`then_1`
      (if (`self.SpawnProjectile`)
        (`|SpawnActorFromClass` "/Game/Blueprints/Weapons/BP_Projectile2.BP_Projectile2_C" (`SceneComponent.K2_GetComponentToWorld` (`self.ProjectileSpawnLocation`)) "Undefined" "OverrideRootScale" null null)
        (set `self.SpawnProjectile` false)
        (`KismetSystemLibrary.Delay` 1.0)
        (set `self.SpawnProjectile` true)))))

(fn `UserConstructionScript`)