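; BP_Enemy_4 is an enemy NPC that roams random navmesh points, chases the player, deals damage on reaching them and fires projectiles.
; BeginPlay starts movement from AIstate and binds to the player's death, which disables sensing and re-runs that state check.
; PawnSensing sightings trigger the chase, face the seen character and spawn a projectile behind a cooldown gate.
; Incoming damage lowers health and destroys the actor at zero.
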(event `self.ReceiveBeginPlay`
  (bind _asbp_fps (cast `/Game/Blueprints/Characters/Player/BP_FPS` (`GameplayStatics.GetPlayerCharacter` 0)))
  (add `/Game/Blueprints/Characters/Player/BP_FPS.PlayerDied` _asbp_fps (delegate `ResetAi`))
  (switch `/Game/Blueprints/Characters/NPCs/E_AIState` (`self.AIstate`) :!label _label
    (:`NewEnumerator0`
      (`self.MoveToRandomLocation`))
    (:`NewEnumerator1`
      (`self.MoveToRandomLocation`))
    (:`NewEnumerator2`
      (`self.ChasePlayer`))))

(event `ResetAi`
  (`PawnSensingComponent.SetSensingUpdatesEnabled` (`self.PawnSensing`) false)
  (goto _label))

(event `self.ReceiveAnyDamage`
  (params (Damage :type "Float (single-precision)") (DamageType :type "DamageType Object Reference") (InstigatedBy :type "Controller Object Reference") (DamageCauser :type "Actor Object Reference"))
  ;[1 1 1] dano
  (if (> (`self.CurrentHealth`) 0.0)
    (bind _output_get (set `self.CurrentHealth` (- (`self.CurrentHealth`) Damage)))
    (if (<= _output_get 0.0)
      (`self.K2_DestroyActor`))))

(event `ChasePlayer`
  (set `CharacterMovementComponent.MaxWalkSpeed` 500.0 (`self.CharacterMovement`))
  (if (`PawnSensingComponent.bEnableSensingUpdates` (`self.PawnSensing`))
    (`|AIMoveTo` self (0.0 0.0 0.0) (`GameplayStatics.GetPlayerCharacter` 0)
      (:`OnSuccess`
        (bind _asbp_fps (cast `/Game/Blueprints/Characters/Player/BP_FPS` (`GameplayStatics.GetPlayerCharacter` 0)))
        (`GameplayStatics.ApplyDamage` _asbp_fps (`self.AppliedDamage`))
        (`KismetSystemLibrary.Delay` 2.0)
        (`self.ChasePlayer`))
      (:`OnFail`
        (`self.MoveToRandomLocation`)
        (set `CharacterMovementComponent.MaxWalkSpeed` 600.0 (`self.CharacterMovement`))))))

(event `MoveToRandomLocation`
  (set `CharacterMovementComponent.MaxWalkSpeed` 200.0 (`self.CharacterMovement`))
  (`|AIMoveTo` self (`NavigationSystemV1.K2_GetRandomLocationInNavigableRadius` (`self.K2_GetActorLocation`) 1000.0 null null) null
    (:`OnSuccess`
      (`KismetSystemLibrary.Delay` 2.0)
      (`self.MoveToRandomLocation`))))

(event `self.PawnSensing.OnSeePawn`
  (params (Pawn :type "Pawn Object Reference"))
  (`self.ChasePlayer`)
  (bind _ascharacter (cast `Character` Pawn))
  (`|ExecutionSequence`
    (:`then_0`
      (`self.K2_SetActorRotation` (`KismetMathLibrary.FindLookAtRotation` (`self.K2_GetActorLocation`) (`self.K2_GetActorLocation` _ascharacter))))
    (:`then_1`
      (if (`self.SpawnProjectile`)
        (`|SpawnActorFromClass` "/Game/Blueprints/Weapons/BP_FirstPersonProjectile.BP_FirstPersonProjectile_C" (`SceneComponent.K2_GetComponentToWorld` (`self.ProjectileSpawnLocation`)) "Undefined" "OverrideRootScale" null null)
        (set `self.SpawnProjectile` false)
        (`KismetSystemLibrary.Delay` 0.8)
        (set `self.SpawnProjectile` true)))))

(fn `UserConstructionScript`)