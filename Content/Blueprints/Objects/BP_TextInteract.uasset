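; BP_TextInteract is an interactable object that shows a text dialog on screen.
; Its Interact event toggles the dialog: an existing UI_Dialog widget is removed and cleared, otherwise one is created for player 0 and added to the viewport.
; The object's MyText variable fills the widget's DialogueText, set just after it is added to the viewport.
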(event `/Game/Blueprints/HUD/Dialogue/BP_DialogInterface.Interact`
  (`/Engine/EditorBlueprintResources/StandardMacros.IsValid` (`self.UIDialogRef`)
    (:`Is Valid`
      (`Widget.RemoveFromParent` (`self.UIDialogRef`))
      (set `self.UIDialogRef` null))
    (:`Is Not Valid`
      (bind _returnvalue (`|CreateWidget` "/Game/Blueprints/HUD/Dialogue/UI_Dialog.UI_Dialog_C" (`GameplayStatics.GetPlayerController` 0)))
      (bind _output_get (set `self.UIDialogRef` _returnvalue))
      (`UserWidget.AddToViewport` _output_get 0)
      (set `/Game/Blueprints/HUD/Dialogue/UI_Dialog.DialogueText` (`self.MyText`) (`self.UIDialogRef`)))))

(fn `UserConstructionScript`)