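; Lockable hinged door that needs a matching key from the player's inventory to open.
; OpenDoors looks up KeyRef on BP_FPS, prints a locked message if missing, otherwise consumes the key and unlocks permanently.
; It infers open or closed from Door1's current rotation, ignoring calls away from those end positions.
; Timelines lerp the door to either side, chosen by DoorDirection, or back to closed.
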(event `self.ReceiveBeginPlay`
  (set `self.Door1Origin` (`SceneComponent.RelativeRotation` (`self.Door1`))))

(event `OpenDoors`
  (if (`self.Locked`)
    (bind _asbp_fps (cast `/Game/Blueprints/Characters/Player/BP_FPS` (`GameplayStatics.GetPlayerCharacter` 0)))
    (bind _returnvalue (`KismetArrayLibrary.Array_Find` (`/Game/Blueprints/Characters/Player/BP_FPS.Inventory` _asbp_fps) (`self.KeyRef`)))
    (if (== _returnvalue -1)
      (`KismetSystemLibrary.PrintString` "Door Locked")
      (else
        (set `self.Locked` false)
        (`/Game/Blueprints/Characters/Player/BP_FPS.RemoveItem` _asbp_fps _returnvalue)
        (set `self.RotacionActual` (`SceneComponent.RelativeRotation` (`self.Door1`)) :!label _label)
        (if (== (`self.RotacionActual`) (struct) :`ErrorTolerance` 1.0)
          (set `self.ClosedDoor` true)
          (set `self.OpenDoor` false)
          (if (`self.ClosedDoor`) :!label _label_2
            (if (`self.DoorDirection`)
              (bind (_direction _newtrack_1) (`Timeline|0to1` :!via `PlayFromStart`)
                (:`Update`
                  (bind _returnvalue_2 (`KismetMathLibrary.RLerp` (`self.Door1Origin`) (struct :`Yaw` -90.0) _newtrack_1 true))
                  (`SceneComponent.K2_SetRelativeRotation` (`self.Door1`) _returnvalue_2 false false))
                (:`Finished`
                  (set `self.Door1Origin` _returnvalue_2)))
              (else
                (bind (_direction_2 _newtrack_1_2) (`Timeline|Timeline_0` :!via `PlayFromStart`)
                  (:`Update`
                    (bind _returnvalue_3 (`KismetMathLibrary.RLerp` (`self.Door1Origin`) (struct :`Yaw` 90.0) _newtrack_1_2 true))
                    (`SceneComponent.K2_SetRelativeRotation` (`self.Door1`) _returnvalue_3 false false))
                  (:`Finished`
                    (set `self.Door1Origin` _returnvalue_3)))))
            (else
              (bind (_direction_3 _newtrack_1_3) (`Timeline|Timeline_1` :!via `PlayFromStart`)
                (:`Update`
                  (bind _returnvalue_4 (`KismetMathLibrary.RLerp` (`self.Door1Origin`) (struct) _newtrack_1_3 true))
                  (`SceneComponent.K2_SetRelativeRotation` (`self.Door1`) _returnvalue_4 false false))
                (:`Finished`
                  (set `self.Door1Origin` _returnvalue_4)))))
          (elif (== (`self.RotacionActual`) (struct :`Yaw` -89.0) :`ErrorTolerance` 1.0)
            (set `self.OpenDoor` true :!label _label_3)
            (set `self.ClosedDoor` false)
            (goto _label_2)
            (elif (== (`self.RotacionActual`) (struct :`Yaw` 89.0) :`ErrorTolerance` 1.0)
              (goto _label_3))))))
    (else
      (goto _label))))

(fn `UserConstructionScript`)